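; Player controller for the BolasLocas game that manages the UI flow from difficulty menu to HUD to win or lose screen.
; It shows WBP_MenuDificultad on begin play; IniciarUI swaps in the player HUD, calls SetearVariables on GM_BolasLocas and copies current and target score into the HUD.
; ActualizarViewPort refreshes the score, while win and lose events show their widgets and pause the game with UI-only input.
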(event Custom|ActualizarViewPort
  (params (Actual :type Integer))
  (bind _playeruiref (Variables|Default|GetPlayerUIREF))
  ;[0 0 0] Actualiza el valor del puntaje
  (Utilities|IsValid _playeruiref
    (:Is%20Valid
      (Variables|/Game/05_UI/WBP_PlayerUI.WBP_PlayerUI_C|SetCantidadActual _playeruiref Actual))))

(event Custom|GanoElJuego
  ;[0 0 0] Eventos Ganar/Perder
  (Viewport|RemoveAllWidgets)
  (bind _returnvalue (UserInterface|CreateWidget "/Game/05_UI/WBP_WinUI.WBP_WinUI_C"))
  (UserInterface|Viewport|AddtoViewport _returnvalue 0)
  (Input|SetInputModeUIOnly self 0 "DoNotLock" false)
  (Variables|Default|SetbShowMouseCursor true)
  (Game|SetGamePaused true))

(event Custom|PerdioEl%20juego
  ;[0 0 0] Eventos Ganar/Perder
  (Viewport|RemoveAllWidgets)
  (bind _returnvalue (UserInterface|CreateWidget "/Game/05_UI/WBP_LoseUI.WBP_LoseUI_C"))
  (UserInterface|Viewport|AddtoViewport _returnvalue 0)
  (Input|SetInputModeUIOnly self 0 "DoNotLock" false)
  (Variables|Default|SetbShowMouseCursor true)
  (Game|SetGamePaused true))

(event Custom|IniciarUI
  ;[0 0 0] Inicializacion de UI
  (Game|SetGamePaused false)
  (Viewport|RemoveAllWidgets)
  (bind _returnvalue (UserInterface|CreateWidget "/Game/05_UI/WBP_PlayerUI.WBP_PlayerUI_C"))
  (bind _output_get (Variables|Default|SetPlayerUIREF _returnvalue))
  (UserInterface|Viewport|AddtoViewport _output_get 0)
  (Input|SetInputModeGameOnly self false)
  (Variables|Default|SetbShowMouseCursor false)
  ;[0 0 0] Set Variables al principio del nivel
  (bind _asgm_bolas_locas (Utilities|Casting|CastToGM_BolasLocas (Game|GetGameMode)))
  (Default|SetearVariables _asgm_bolas_locas)
  (Utilities|IsValid (Variables|Default|GetPlayerUIREF)
    (:Is%20Valid
      (Variables|/Game/05_UI/WBP_PlayerUI.WBP_PlayerUI_C|SetCantidadActual (Variables|Default|GetPlayerUIREF) (Variables|/Game/01_Core/GM_BolasLocas.GM_BolasLocas_C|GetPuntajeActual _asgm_bolas_locas))
      (Variables|/Game/05_UI/WBP_PlayerUI.WBP_PlayerUI_C|SetCantidadGanar (Variables|Default|GetPlayerUIREF) (Variables|/Game/01_Core/GM_BolasLocas.GM_BolasLocas_C|GetPuntajeParaGanar _asgm_bolas_locas)))))

(event EventBeginPlay
  ;[0 0 0] Menu elegir dificultad
  (bind _returnvalue (UserInterface|CreateWidget "/Game/05_UI/WBP_MenuDificultad.WBP_MenuDificultad_C"))
  (UserInterface|Viewport|AddtoViewport _returnvalue 0)
  (Game|SetGamePaused false)
  (Input|SetInputModeUIOnly self 0 "DoNotLock" false)
  (Variables|Default|SetbShowMouseCursor true))

(fn ConstructionScript)