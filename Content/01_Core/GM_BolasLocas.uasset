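; Game mode for Bolas Locas that keeps the score, decides win or loss, and can restart Level_01.
; SetearVariables resets the score, loads thresholds and spawn time from the GameInstance's selected difficulty (lose threshold from Cant_Ganar, win from Cant_Perder), then refreshes the first BP_BolasSpawner.
; SetearPuntaje checks each new total against both thresholds, telling the PlayerController to show win, loss, or the updated score.
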(event Custom|ReiniciarNivel
  ;[0 0 0] Reiniciar Nivel
  (Game|OpenLevel(byName) "Level_01"))

(event Custom|SetearPuntaje
  (params (Cantidad :type Integer))
  ;[0 0 0] Setear Puntaje
  ;;[0 0 0] CheckWin
  (if (>= (+ Cantidad (Variables|Default|GetPuntajeActual)) (Variables|Default|GetPuntajeParaGanar))
    (bind _aspc_bolas_locas (Utilities|Casting|CastToPC_BolasLocas (Game|GetPlayerController 0)))
    (Default|GanoElJuego _aspc_bolas_locas)
    (else
      ;;[0 0 0] CheckWin
      (if (<= (+ Cantidad (Variables|Default|GetPuntajeActual)) (Variables|Default|GetPuntajeParaPerder))
        (bind _aspc_bolas_locas_2 (Utilities|Casting|CastToPC_BolasLocas (Game|GetPlayerController 0)))
        (Default|PerdioElJuego _aspc_bolas_locas_2)
        (else
          ;;[0 0 0] SetNewPoints
          (bind _output_get (Variables|Default|SetPuntajeActual (+ (Variables|Default|GetPuntajeActual) Cantidad)))
          (bind _aspc_bolas_locas_3 (Utilities|Casting|CastToPC_BolasLocas (Game|GetPlayerController 0)))
          (Default|ActualizarViewPort _aspc_bolas_locas_3 _output_get))))))

(event Custom|SetearVariables
  ;[0 0 0] Set Variables DataDriven
  (bind _asgi_bolas_locas (Utilities|Casting|CastToGI_BolasLocas (Game|GetGameInstance)))
  (Variables|Default|SetPuntajeActual 0)
  (Variables|Default|SetTiempoSpawn (.spawntime (Variables|/Game/01_Core/GI_BolasLocas.GI_BolasLocas_C|GetDificultadSelect _asgi_bolas_locas)))
  (Variables|Default|SetPuntajeParaPerder (.cant_ganar (Variables|/Game/01_Core/GI_BolasLocas.GI_BolasLocas_C|GetDificultadSelect _asgi_bolas_locas)))
  (Variables|Default|SetPuntajeParaGanar (.cant_perder (Variables|/Game/01_Core/GI_BolasLocas.GI_BolasLocas_C|GetDificultadSelect _asgi_bolas_locas)))
  ;[0 0 0] Actualizar el tiempo de spawn
  (bind _outactors (Actor|GetAllActorsOfClass "/Game/03_Blueprints/BP_BolasSpawner.BP_BolasSpawner_C"))
  (if (> (Utilities|Array|Length _outactors) 0)
    (Default|ActualizarTiempoSpawn (Utilities|Array|Get(acopy) _outactors))))

(fn ConstructionScript)