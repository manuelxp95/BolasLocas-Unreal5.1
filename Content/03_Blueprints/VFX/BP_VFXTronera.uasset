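; BP_VFXTronera is a VFX actor for a "tronera" that shows a color-specific particle effect for a set time.
; On BeginPlay, it looks up ColorID in the Colores map and, if found, assigns that template to its four particle system components.
; ActivarParticulas makes all four visible, waits for the given Delay, then hides them, toggling visibility rather than activating or deactivating the systems.
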(event Custom|ActivarParticulas
  (params (Delay :type Float%20%28double-precision%29))
  (bind _particlesystem1 (Variables|Default|GetParticleSystem1))
  ;[0 0 0] ActivamosVFX
  (Rendering|SetVisibility _particlesystem1 true false)
  (Utilities|FlowControl|Delay Delay)
  (Rendering|SetVisibility _particlesystem1 false false))

(event EventBeginPlay
  (bind _colores (Variables|Default|GetColores))
  (bind _colorid (Variables|Default|GetColorID))
  (bind (_value _returnvalue) (Utilities|Map|Find _colores _colorid))
  ;[0 0 0] Seteo Inicial de particulas
  (if _returnvalue
    (Effects|Components|ParticleSystem|SetTemplate (Variables|Default|GetParticleSystem3) _value)))

(fn ConstructionScript)