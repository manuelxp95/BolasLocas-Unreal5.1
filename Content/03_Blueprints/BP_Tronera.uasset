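; BP_Tronera is a colour-coded pocket (tronera) that scores balls and kills the player on overlap.
; Its Box overlap calls OnPlayerDeath on the player's character after a short delay.
; For a BP_BolaLoca, it compares ColorID with TroneraColorID, adds or subtracts a point through GM_BolasLocas.SetearPuntaje, then destroys the ball.
; A match also triggers particles on the referenced BP_VFXTronera, whose failed cast skips the ball's destruction.
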(event OnComponentBeginOverlap(Box)
  (params (OverlappedComponent :type Primitive%20Component%20Object%20Reference) (OtherActor :type Actor%20Object%20Reference) (OtherComp :type Primitive%20Component%20Object%20Reference) (OtherBodyIndex :type Integer) (bFromSweep :type Boolean) (SweepResult :type Hit%20Result%20Structure%20%28by%20ref%29))
  ;[0 0 0] Ingresa un obj a la tronera
  ;;[0 0 0] PersonajeCheck
  (if (== OtherActor (Game|Player|GetPlayerPawn 0))
    ;;[0 0 0] Reiniciar Nivel
    (Utilities|FlowControl|Delay 0.5)
    (bind _asbp_third_person_character (Utilities|Casting|CastToBP_ThirdPersonCharacter OtherActor))
    (Default|OnPlayerDeath _asbp_third_person_character)
    (else
      ;;[0 0 0] CheckBola
      (if (== (Utilities|GetClass OtherActor) "/Game/03_Blueprints/BP_BolaLoca.BP_BolaLoca_C")
        (bind _asbp_bola_loca (Utilities|Casting|CastToBP_BolaLoca OtherActor))
        (if (== (Variables|Default|GetTroneraColorID) (Variables|/Game/03_Blueprints/BP_BolaLoca.BP_BolaLoca_C|GetColorID _asbp_bola_loca))
          (bind _asgm_bolas_locas (Utilities|Casting|CastToGM_BolasLocas (Game|GetGameMode)))
          (Default|SetearPuntaje _asgm_bolas_locas 1)
          (bind _asbp_vfxtronera (Utilities|Casting|CastToBP_VFXTronera (Variables|Default|GetVfxActorREF))
            (:then
              (Default|ActivarParticulas _asbp_vfxtronera 2.0))
            (:CastFailed
              _))
          (else
            (bind _asgm_bolas_locas_2 (Utilities|Casting|CastToGM_BolasLocas (Game|GetGameMode)))
            (Default|SetearPuntaje _asgm_bolas_locas_2 -1)))
        (Default|DestruirBola _asbp_bola_loca)))))

(fn ConstructionScript)