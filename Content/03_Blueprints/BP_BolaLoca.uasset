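; BP_BolaLoca is a ball actor that takes a random color when spawned and can destroy itself.
; On BeginPlay it picks a random integer key from 1 to the size of the Colores map, stores it as ColorID and applies the matching material to its sphere.
; The DestruirBola event destroys the actor after a short delay; nothing in this file calls it.
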(event Custom|DestruirBola
  ;[0 0 0] AutoDestructor
  (Utilities|FlowControl|Delay 1.0)
  (Actor|DestroyActor))

(event EventBeginPlay
  ;[0 0 0] BeginPlay - SetColor
  (bind _output_get (Variables|Default|SetColorID (Math|Random|RandomIntegerinRange 1 (Utilities|Map|Length (Variables|Default|GetColores)))))
  (Rendering|Material|SetMaterial (Variables|Default|GetSphere) 0 (.Value (Utilities|Map|Find (Variables|Default|GetColores) _output_get))))

(fn ConstructionScript)