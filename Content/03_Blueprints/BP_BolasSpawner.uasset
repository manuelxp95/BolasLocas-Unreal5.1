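; BP_BolasSpawner is a spawner actor that repeatedly creates BP_BolaLoca actors at its own location and rotation.
; On BeginPlay it reads the spawn interval, TiempoSpawn, from the GM_BolasLocas game mode.
; Tick feeds a Delay scaled by that interval and frame time, so the pending delay throttles spawning into a periodic loop.
; Each spawned ball gets a uniform scale from SpawnSize.
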(event EventBeginPlay
  (bind _asgm_bolas_locas (Utilities|Casting|CastToGM_BolasLocas (Game|GetGameMode)))
  (Variables|Default|SetTiempo (Variables|/Game/01_Core/GM_BolasLocas.GM_BolasLocas_C|GetTiempoSpawn _asgm_bolas_locas)))

(event EventTick
  (params (DeltaSeconds :type Float%20%28single-precision%29))
  (bind _returnvalue (Transformation|GetActorTransform))
  (bind _spawnsize (Variables|Default|GetSpawnSize))
  (Utilities|FlowControl|Delay (* (+ DeltaSeconds 1.0) (Variables|Default|GetTiempo)))
  (Game|SpawnActorfromClass "/Game/03_Blueprints/BP_BolaLoca.BP_BolaLoca_C" (Math|Transform|MakeTransform (.location _returnvalue) (.rotation _returnvalue) (Math|Vector|MakeVector _spawnsize _spawnsize _spawnsize)) "Undefined" 0 0))

(fn ConstructionScript)